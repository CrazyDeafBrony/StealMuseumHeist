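; TutorialPickup is a collectible actor that rewards the player with score and extra countdown time.
; When its static mesh begins overlapping a FirstPersonCharacter, it increments that character's ScoreSet and destroys itself.
; It then extends the CountdownTimer on MyGameState and plays a cash register sound at the world origin rather than at the pickup's position.
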(event OnComponentBeginOverlap(StaticMesh)
  (params (OtherActor :type Actor%20Object%20Reference) (OtherComp :type Primitive%20Component%20Object%20Reference) (OtherBodyIndex :type Integer) (bFromSweep :type Boolean) (SweepResult :type Hit%20Result%20Structure%20%28by%20ref%29))
  (bind _asfirst_person_character (Utilities|Casting|CastToFirstPersonCharacter OtherActor))
  (Variables|/Game/FirstPersonBP/Blueprints/FirstPersonCharacter.FirstPersonCharacter_C|SetScoreSet _asfirst_person_character (+ (Variables|/Game/FirstPersonBP/Blueprints/FirstPersonCharacter.FirstPersonCharacter_C|GetScoreSet _asfirst_person_character) 1))
  (Actor|DestroyActor)
  (bind _asmy_game_state (Utilities|Casting|CastToMyGameState (Game|GetGameState)))
  (Variables|/Game/FirstPersonBP/Blueprints/MyGameState.MyGameState_C|SetCountdownTimer _asmy_game_state (+ (Variables|/Game/FirstPersonBP/Blueprints/MyGameState.MyGameState_C|GetCountdownTimer _asmy_game_state) 15.0))
  (Audio|PlaySoundatLocation "/Game/Blueprints/Cha_Ching_Register-Muska666-173262285.Cha_Ching_Register-Muska666-173262285" "0, 0, 0"))

(event EventBeginPlay)

(event EventActorBeginOverlap
  (params (OtherActor :type Actor%20Object%20Reference)))

(event EventTick
  (params (DeltaSeconds :type Float%20%28single-precision%29)))

(fn ConstructionScript)